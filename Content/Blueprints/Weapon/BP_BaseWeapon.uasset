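; Base weapon Blueprint for BP_Player, handling hitscan firing, magazine reloads and ammo HUD updates.
; WeaponFire plays montages, spends ammo, spawns a Niagara tracer and damages BP_BaseEnemy with head-bone criticals, looping after FireRate for one WeaponType until stopped or empty.
; LineTraceLogic traces from the camera view with random spread, retracing from the muzzle if that target lies behind it.
; WeaponReload refills the magazine from reserve ammo, re-enabling fire when the montage completes.
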(event Custom|WeaponFire
  (bind _hitreult (Variables|Default|GetHitReult))
  (if (not (Variables|/Game/Blueprints/Player/BP_Player.BP_Player_C|GetIsStopFire (Variables|Default|GetPlayerRef))) :!label _label
    (Variables|Default|SetCanFire false)
    (Animation|Montage|PlayMontage (Variables|/Script/Engine.Character|GetMesh (Variables|Default|GetPlayerRef)) (Variables|AnimMontage|GetFairAnim)
      (:then
        (Animation|Montage|PlayMontage (Variables|Default|GetWeaponMesh) (Variables|AnimMontage|GetFireWeaponAnim)
          (:then
            (CallFunction|UpdateAmmoMagazine)
            (Default|UpdateAmmoInfo (Variables|UI|GetWeaponWidgetRef) (Variables|Ammo|GetCurrentAmmo) (Variables|Ammo|GetAmmoMagazine))
            (bind _hitreult_2 (CallFunction|LineTraceLogic))
            (CallFunction|TraceandPoint _hitreult_2)
            (CallFunction|TraceFX)
            (bind _asbp_base_enemy (Utilities|Casting|CastToBP_BaseEnemy (.hitactor _hitreult))
              (:then
                (Game|Damage|ApplyDamage _asbp_base_enemy (Math|Float|SelectFloat (Variables|Default|GetCriticalDamage) (Variables|Default|GetDamage) (== (.hitbonename _hitreult) "head")) 0 self))
              (:CastFailed
                _))
            (Utilities|FlowControl|Delay (Variables|Ammo|GetFireRate))
            (if (Variables|Ammo|GetMagazineEmpty)
              (Variables|Default|SetCanFire false)
              (Development|PrintString "Ammo Is NULL")
              (else
                (Variables|Default|SetCanFire true)
                (if (Utilities|Enum|Equal(Enum) (Variables|Default|GetWeaponType) "NewEnumerator1")
                  (goto _label))))))))))

(event Custom|WeaponReload
  (if (and (CallFunction|AmmoNotEmpty) (not (CallFunction|MagazineFull)))
    (Variables|Default|SetIsReload true)
    (CallFunction|CalculateAmmo)
    (Variables|Ammo|SetMagazineEmpty false)
    (Default|UpdateAmmoInfo (Variables|UI|GetWeaponWidgetRef) (Variables|Ammo|GetCurrentAmmo) (Variables|Ammo|GetAmmoMagazine))
    (Animation|Montage|PlayMontage (Variables|/Script/Engine.Character|GetMesh (Variables|Default|GetPlayerRef)) (Variables|AnimMontage|GetReloadAnim)
      (:OnCompleted
        (Variables|Default|SetIsReload false)
        (Variables|Default|SetCanFire true)))))

(event EventBeginPlay
  (bind _asbp_player (Utilities|Casting|CastToBP_Player (Components|GetOwner)))
  (Variables|Default|SetPlayerRef _asbp_player))

(fn ConstructionScript
  (Variables|Ammo|SetCurrentAmmo (Variables|Ammo|GetMaxAmmo)))

(fn AttachtoHand
  (params (HandSocket :type Name))
  (Transformation|AttachComponentToComponent (Variables|/Script/Engine.Character|GetMesh (Variables|Default|GetPlayerRef)) HandSocket "SnapToTarget" "SnapToTarget" "SnapToTarget" true))

(fn SetWeaponWidgetRef
  (params (WeaponWidget :type WBP%20Weapon%20Object%20Reference))
  (Variables|UI|SetWeaponWidgetRef WeaponWidget))

(fn UpdateWidgetInfo
  (Default|UpdateWeaponWidgetInfo (Variables|UI|GetWeaponWidgetRef) (Variables|Ammo|GetCurrentAmmo) (Variables|Ammo|GetAmmoMagazine) (Variables|UI|GetImageHud)))

(fn UpdateAmmoMagazine
  (bind _result (Math|Integer|DecrementInt (Variables|Ammo|GetAmmoMagazine))
    (:%20%20
      (if (== _result 0)
        (Variables|Ammo|SetMagazineEmpty true)))))

(fn LineTraceLogic
  (bind _returnvalue (Game|GetPlayerController 0))
  (bind _muzzlesocket (Variables|Ammo|GetMuzzleSocket))
  (bind _weaponmesh (Variables|Default|GetWeaponMesh))
  (bind _returnvalue_2 (Transformation|GetSocketLocation _weaponmesh _muzzlesocket))
  (bind (_location _rotation) (Pawn|GetPlayerViewPoint _returnvalue))
  (bind _outhit (Collision|LineTraceByChannel _location (Math|Random|RandomPointinBoundingBox (+ _location (* (Math|Rotator|GetRotationXVector _rotation) (Variables|Ammo|GetFireDistance))) (* "1.000000,1.000000,1.000000" (Variables|Ammo|GetSpread))) "TraceTypeQuery1" false 0 "None"))
  (if true
    _
    (else
      _))
  (Variables|Default|SetHitReult _outhit)
  (if (> (Class|KismetMathLibrary|DegAcos (Math|Vector|DotProduct (Math|Vector|GetForwardVector (Transformation|GetSocketRotation (Variables|Default|GetWeaponMesh) (Variables|Ammo|GetMuzzleSocket))) (- (Math|Vector|SelectVector (.ImpactPoint (Collision|BreakHitResult _outhit)) (.TraceEnd (Collision|BreakHitResult _outhit)) (.bBlockingHit (Collision|BreakHitResult _outhit))) (Transformation|GetSocketLocation (Variables|Default|GetWeaponMesh) (Variables|Ammo|GetMuzzleSocket))))) 9e+01)
    (bind _outhit_2 (Collision|LineTraceByChannel _returnvalue_2 (Math|Random|RandomPointinBoundingBox (+ _returnvalue_2 (* (Math|Vector|GetForwardVector (Transformation|GetSocketRotation (Variables|Default|GetWeaponMesh) (Variables|Ammo|GetMuzzleSocket))) (Variables|Ammo|GetFireDistance))) (* "1.000000,1.000000,1.000000" (Variables|Ammo|GetSpread))) "TraceTypeQuery1" false 0 "None"))
    (bind _output_get (Variables|Default|SetHitReult _outhit_2))
    (return _output_get)
    (else
      (return (Variables|Default|GetHitReult)))))

(fn TraceandPoint
  (params (HitResult :type Hit%20Result%20Structure))
  (bind (_bblockinghit _binitialoverlap _time _distance _location _impactpoint _normal _impactnormal _physmat _hitactor _hitcomponent _hitbonename _bonename _hititem _elementindex _faceindex _tracestart _traceend) (Collision|BreakHitResult HitResult))
  (if _bblockinghit
    (Variables|Default|SetEndLine _impactpoint)
    (else
      (Variables|Default|SetEndLine _traceend))))

(fn TraceFX
  (bind _returnvalue (Niagara|SpawnSystematLocation (Variables|Default|GetTraceFXSystem) (Transformation|GetSocketLocation (Variables|Default|GetWeaponMesh) (Variables|Ammo|GetMuzzleSocket))))
  (Niagara|SetNiagaraVariable(Vector3) _returnvalue "TraceTarget" (Variables|Default|GetEndLine)))

(fn AmmoNotEmpty
  (return (> (Variables|Ammo|GetCurrentAmmo) 0)))

(fn MagazineFull
  (return (== (Variables|Ammo|GetAmmoMagazine) (Variables|Ammo|GetMaxAmmoMagazine))))

(fn CalculateAmmo
  (if (< (Variables|Ammo|GetCurrentAmmo) (- (Variables|Ammo|GetMaxAmmoMagazine) (Variables|Ammo|GetAmmoMagazine)))
    (Variables|Ammo|SetAmmoMagazine (+ (Variables|Ammo|GetCurrentAmmo) (Variables|Ammo|GetAmmoMagazine)))
    (Variables|Ammo|SetCurrentAmmo 0)
    (else
      (bind _output_get (LocalVariables|SetAddMagazineAmmo (- (Variables|Ammo|GetMaxAmmoMagazine) (Variables|Ammo|GetAmmoMagazine))))
      (Variables|Ammo|SetAmmoMagazine (+ _output_get (Variables|Ammo|GetAmmoMagazine)))
      (Variables|Ammo|SetCurrentAmmo (- (Variables|Ammo|GetCurrentAmmo) (LocalVariables|GetAddMagazineAmmo))))))