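; Health component that tracks its owner's current health, starting at max on BeginPlay, with damage and heal events.
; Lethal damage zeroes health and sends a death message to the owner; healing clamps at max.
; It gets the HUD health bar through the owner's player-reference message.
; Heal sets the bar to the health fraction, while damage to a BP_Player sets it to zero, leaving the ratio calculation unused.
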(event Custom|TakeDamage
  (params (Damage :type Float%20%28double-precision%29))
  (if (<= (- (Variables|Default|GetCurrentHealth) Damage) 0.0)
    (Variables|Default|SetCurrentHealth 0.0)
    (Class|BPIHelperHealthComponent|OnDeath(Message) (Components|GetOwner))
    (else
      (bind _output_get (Variables|Default|SetCurrentHealth (- (Variables|Default|GetCurrentHealth) Damage)))))
  (if (.bSuccess (Utilities|Casting|CastToBP_Player (Components|GetOwner)))
    (Default|SetHealth (Variables|Default|GetHealthWidgetRef) 0.0)))

(event Custom|Heal
  (params (Amount :type Float%20%28double-precision%29))
  (bind _output_get (Variables|Default|SetCurrentHealth (Math|Float|Clamp(Float) (+ Amount (Variables|Default|GetCurrentHealth)) (Variables|Default|GetCurrentHealth) (Variables|Default|GetMaxHealth))))
  (Default|SetHealth (Variables|Default|GetHealthWidgetRef) (/ _output_get (Variables|Default|GetMaxHealth))))

(event EventBeginPlay
  (Variables|Default|SetCurrentHealth (Variables|Default|GetMaxHealth)))

(event EventHealthBarWidgetRef
  (bind _player (Class|BPIHelperHealthComponent|RefPlayer(Message) (Components|GetOwner)))
  (Variables|Default|SetHealthWidgetRef (Variables|/Game/UI/Widgets/BP_PlayerHUD.BP_PlayerHUD_C|GetHealthBarWidgetRef (Variables|/Game/Blueprints/Player/BP_Player.BP_Player_C|GetPlayerHUDRef _player)))
  (Default|SetHealth (Variables|Default|GetHealthWidgetRef) 1.0))

(fn RefPlayer
  (return 0))